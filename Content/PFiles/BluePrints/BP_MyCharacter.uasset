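; Player character Blueprint with pistol firing, an aiming state and camera shake feedback.
; Fire runs a debug-drawn Visibility line trace forward from FLocation over FireRange, sets ClickedFire without using the hit result, then plays a fire shake.
; Aiming input toggles a boolean on press and release with debug prints.
; Tick starts the walk camera shake every frame the character has nonzero velocity.
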(event EventBeginPlay)

(event Collision|EventActorBeginOverlap
  (params (OtherActor :type Actor%20Object%20Reference)))

(event EventTick
  (params (DeltaSeconds :type Float%20%28single-precision%29))
  ;[1 1 1] CameraShakeWalk
  (if (> (Math|Vector|VectorLength (Transformation|GetVelocity)) 0.0)
    (CallFunction|PlayCameraShakeWalk)))

(event Input|ActionEvents|InputActionFire
  (params (Key :type Key%20Structure :default "None"))
  ;[1 1 1] CameraShake Fire
  (:Pressed
    (CallFunction|FirePistol)
    (CallFunction|PlayCameraShakeFire)))

(event Input|ActionEvents|InputActionAiming
  (params (Key :type Key%20Structure :default "None"))
  (:Pressed
    (Development|PrintString "123" true true "(R=1.000000,G=0.000000,B=0.107647,A=1.000000)")
    (bind _output_get (Variables|Pistol|SetAiming true))
    (Development|PrintString (Utilities|String|ToString(Boolean) _output_get)))
  (:Released
    (bind _output_get_2 (Variables|Pistol|SetAiming false))
    (Development|PrintString (Utilities|String|ToString(Boolean) _output_get_2))))

(fn ConstructionScript)

(fn FirePistol
  (bind _flocation (Variables|Default|GetFLocation))
  (bind _returnvalue (Transformation|GetWorldLocation _flocation))
  (Collision|LineTraceByChannel _returnvalue (+ _returnvalue (* (Math|Vector|GetForwardVector _flocation) (Variables|Pistol|GetFireRange))) "TraceTypeQuery1" false 0 "ForDuration")
  (Variables|Pistol|SetClickedFire true))

(fn PlayCameraShakeFire
  (Class|LegacyCameraShake|StartLegacyCameraShake (Game|GetPlayerCameraManager 0) "/Game/PFiles/Camera/BP_FireCameraShake.BP_FireCameraShake_C" 1.0 "CameraLocal" "0, 0, 0"))

(fn PlayCameraShakeWalk
  (Class|LegacyCameraShake|StartLegacyCameraShake (Game|GetPlayerCameraManager 0) "/Game/PFiles/Camera/BP_WalkCameraShake.BP_WalkCameraShake_C" 1.0 "CameraLocal" "0, 0, 0"))